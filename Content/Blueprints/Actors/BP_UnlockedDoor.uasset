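; BP_UnlockedDoor is a door actor that toggles between open and closed whenever its OpenDoor event is called.
; Separate open and close timelines drive the Door component's relative yaw, with IsOpened selecting which one runs.
; AnimOpenOver and AnimCloseOver flags ignore calls until the current swing finishes.
; Both branches compare OpenDoorAnimation's length and position to choose between Play and PlayFromStart.
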(event EventOpenDoor
  (bind _door (Variables|Default|GetDoor))
  (bind _open_door_animation (Variables|Default|GetOpen%20Door%20Animation))
  (bind _open_door_animation_2 (Variables|Default|GetOpen%20Door%20Animation))
  (if (Variables|Default|GetAnim%20Close%20Over?)
    (if (Variables|Default|GetAnim%20Open%20Over?)
      (if (Variables|Default|GetIs%20opened?)
        (Variables|Default|SetAnim%20Close%20Over? false)
        (Variables|Default|SetIs%20opened? false)
        (if (< (Components|Timeline|GetTimelineLength _open_door_animation) (Components|Timeline|GetPlaybackPosition _open_door_animation))
          (bind _newtrack_0 (Timeline|Close%20Door%20Animation Play)
            (:Update
              (Transformation|SetRelativeRotation _door (Math|Rotator|MakeRotator 0.0 0.0 _newtrack_0) false false))
            (:Finished
              (Variables|Default|SetAnim%20Close%20Over? true)))
          (else
            (Timeline|Close%20Door%20Animation PlayFromStart)))
        (else
          (Variables|Default|SetAnim%20Open%20Over? false)
          (Variables|Default|SetIs%20opened? true)
          (if (< (Components|Timeline|GetTimelineLength _open_door_animation_2) (Components|Timeline|GetPlaybackPosition _open_door_animation_2))
            (bind _newtrack_0_2 (Timeline|Open%20Door%20Animation Play)
              (:Update
                (Transformation|SetRelativeRotation _door (Math|Rotator|MakeRotator 0.0 0.0 _newtrack_0_2) false false))
              (:Finished
                (Variables|Default|SetAnim%20Open%20Over? true)))
            (else
              (Timeline|Open%20Door%20Animation PlayFromStart))))))))

(fn ConstructionScript)